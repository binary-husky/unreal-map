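; Controller Blueprint for a laser launcher agent that handles firing its weapon at a target agent.
; On SpawnWeaponFire it casts the controlled pawn to RLA_LaserLauncher and spawns a Weapon_Laser at that pawn's spawn point.
; The laser receives the target, source agent, team, color, range and damage.
; A failed cast raises a logged error, and construction only calls the parent script.
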(event EventSpawnWeaponFire
  (params (TargetAgent :type Agent%20Object%20Reference))
  (bind _agent (Variables|Default|GetAgent))
  (bind _asrla_laser_launcher (Utilities|Casting|CastToRLA_LaserLauncher (Pawn|GetControlledPawn))
    (:then
      ;[1 1 1] Generate Missile
      (Game|SpawnActorfromClass "/Game/Assets/DefNotAgent/Weapon_Laser.Weapon_Laser_C" (Transformation|GetWorldTransform (Variables|/Game/Assets/DefAgent/Lv1_AgentCanMoveLegacy.Lv1_AgentCanMoveLegacy_C|GetSpawnMsPoint _asrla_laser_launcher)) "AlwaysSpawn" _agent TargetAgent _agent "0.000000,0.000000,1.000000" (Variables|/Game/Assets/AbstractActor/Agent.Agent_C|GetTeamNo _asrla_laser_launcher) (Variables|/Game/Assets/AbstractActor/Agent.Agent_C|GetColor _asrla_laser_launcher) (Variables|Default|GetArg_FireRange) (Variables|Default|GetCombat_MissileDmg) 0))
    (:CastFailed
      (Class|UHMPBlueprintFunctionLibrary|RaiseError "AC_RL:SpawnWeaponFireCastError" true))))

(fn ConstructionScript
  (|CallParentFunction))