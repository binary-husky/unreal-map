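; AI controller for the opposing drone, running its behavior tree with a tagged patrol path bound on the Blackboard.
; On each perception info update, it filters currently perceived actors through IsConcern, which rejects non-agents, the player pawn, owned actors, teammates and flying agents.
; The nearest remaining agent sets CombatMode and InsightActor; none clears both.
; The older per-target perception handler is largely disabled.
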(event OnTargetPerceptionUpdated(AIPerception)
  (params (Actor :type Actor%20Object%20Reference) (Stimulus :type AI%20Stimulus%20Structure))
  (bind _self self)
  (bind _blackboard (Variables|Default|GetBlackboard))
  (bind _returnvalue (Pawn|GetControlledPawn _self))
  (bind _asagent (Utilities|Casting|CastToAgent Actor))
  (bind _asagent_2 (Utilities|Casting|CastToAgent _returnvalue)
    (:then
      (if (not (Math|Boolean|ORBoolean (== Actor (Game|Player|GetPlayerPawn 0)) (== (Components|GetOwner Actor) _returnvalue) (== (Variables|/Game/Assets/AbstractActor/Agent.Agent_C|GetTeamNo _asagent) (Variables|/Game/Assets/AbstractActor/Agent.Agent_C|GetTeamNo _asagent_2))))
        (Development|PrintString "Update Perception" true true "(R=0.000000,G=0.660000,B=1.000000,A=1.000000)" 1e+01)
        (AI|Components|Blackboard|SetValueasBool _blackboard (Utilities|Name|MakeLiteralName "CombatMode") true)
        ;[1 1 1] CombatMode开关：别忘了设置BBK值
        (AI|Components|Blackboard|SetValueasObject _blackboard (Utilities|Name|MakeLiteralName "InsightActor") Actor)))
    (:CastFailed
      (Class|UHMPBlueprintFunctionLibrary|RaiseError "drone is not agent, wtf?" true))))

(event OnTargetPerceptionInfoUpdated(AIPerception)
  (params (UpdateInfo :type Actor%20Perception%20Update%20Info%20Structure%20%28by%20ref%29))
  (bind _blackboard (Variables|Default|GetBlackboard))
  (bind _blackboard_2 (Variables|Default|GetBlackboard))
  (Utilities|Array|Clear (Variables|Default|GetConcernedActors))
  (Variables|Default|SetNearestConcernActor 0)
  (Variables|Default|SetNearestConcernActorDis 10000000272564224.0)
  ;[1 1 1] load concerned agents
  (for _array_element (Class|AIPerceptionComponent|GetCurrentlyPerceivedActors (Variables|Default|GetAIPerception))
    ;[1 1 1] for body
    (bind _concern (CallFunction|IsConcern _array_element))
    (if _concern
      (Utilities|Array|Add (Variables|Default|GetConcernedActors) _array_element)
      ;;[1 1 1] loop to find the nearest agent
      (if (< (Math|Vector|Distance(Vector) (Transformation|GetActorLocation _array_element) (Transformation|GetWorldLocation (Variables|/Script/Engine.Actor|GetRootComponent (Pawn|GetControlledPawn)))) (Variables|Default|GetNearestConcernActorDis))
        (Variables|Default|SetNearestConcernActorDis (Math|Vector|Distance(Vector) (Transformation|GetActorLocation _array_element) (Transformation|GetWorldLocation (Variables|/Script/Engine.Actor|GetRootComponent (Pawn|GetControlledPawn)))))
        (Variables|Default|SetNearestConcernActor _array_element))))
  (if (== (Utilities|Array|Length (Variables|Default|GetConcernedActors)) 0)
    ;[1 1 1] clear combat mode and attack target
    (AI|Components|Blackboard|SetValueasBool _blackboard (Utilities|Name|MakeLiteralName "CombatMode") false)
    (AI|Components|Blackboard|SetValueasObject _blackboard (Utilities|Name|MakeLiteralName "InsightActor") 0)
    (else
      (Utilities|IsValid (Variables|Default|GetNearestConcernActor)
        (:Is%20Valid
          ;[1 1 1] CombatMode开关：别忘了设置BBK值
          (AI|Components|Blackboard|SetValueasBool _blackboard_2 (Utilities|Name|MakeLiteralName "CombatMode") true)
          ;[1 1 1] CombatMode开关：别忘了设置BBK值
          (AI|Components|Blackboard|SetValueasObject _blackboard_2 (Utilities|Name|MakeLiteralName "InsightActor") (Variables|Default|GetNearestConcernActor)))
        (:Is%20Not%20Valid
          (Class|UHMPBlueprintFunctionLibrary|RaiseError "Should be valid" true))))))

(event EventBeginPlay
  (AI|RunBehaviorTree "/Game/Assets/Trashbin/DroneAgentBlueprint/BT_Drone_Opp.BT_Drone_Opp")
  ;[1 1 1] 绑定路径
  (bind _outactors (Actor|GetAllActorsOfClasswithTag "/Game/Assets/Trashbin/DroneAgentBlueprint/LinkingPointGroup.LinkingPointGroup_C" "opp_patrol_road"))
  (AI|Components|Blackboard|SetValueasObject (Variables|Default|GetBlackboard) (Utilities|Name|MakeLiteralName "Path") (Utilities|Array|Get(acopy) _outactors)))

(fn ConstructionScript)

(fn IsConcern
  (params (obs_actor :type Actor%20Object%20Reference))
  (bind _self self)
  (bind _returnvalue (Pawn|GetControlledPawn _self))
  (bind _asagent (Utilities|Casting|CastToAgent obs_actor)
    (:then
      (bind _asagent_2 (Utilities|Casting|CastToAgent _returnvalue)
        (:then
          (if (Math|Boolean|ORBoolean (== obs_actor (Game|Player|GetPlayerPawn 0)) (== (Components|GetOwner obs_actor) _returnvalue) (== (Variables|/Game/Assets/AbstractActor/Agent.Agent_C|GetTeamNo _asagent) (Variables|/Game/Assets/AbstractActor/Agent.Agent_C|GetTeamNo _asagent_2)))
            _
            (else
              (Utilities|IsValid _asagent
                (:Is%20Valid
                  (if (Class|NavMovementComponent|IsFlying (Variables|/Script/Engine.Character|GetCharacterMovement _asagent))
                    (return false)
                    (else
                      (return true))))
                (:Is%20Not%20Valid
                  _)))))
        (:CastFailed
          (Class|UHMPBlueprintFunctionLibrary|RaiseError "drone is not agent, wtf?" true))))
    (:CastFailed
      _))
  (return false))